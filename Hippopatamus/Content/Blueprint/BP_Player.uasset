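; BP_Player is the player Blueprint that feeds its location to an enemy AI every Tick.
; It casts the controller of the referenced MyEmemy to BP_AI_ENEMY_CONTROLLER, calls UseBlackboard with BB_ENEMY_BEHAVIOR each frame, and writes its location to the PlayerLocation key.
; Debug prints show its name each frame and, when the cast succeeds, its location.
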(event `self.ReceiveBeginPlay`)

(event `self.ReceiveTick`
  (params (DeltaSeconds :type "Float (single-precision)"))
  (bind _returnvalue (`self.K2_GetActorLocation`))
  (`KismetSystemLibrary.PrintString` (`KismetSystemLibrary.GetDisplayName` self))
  (bind _asbp_ai_enemy_controller (cast `/Game/Blueprint/enemy_AI_BP/BP_AI_ENEMY_CONTROLLER` (`self.GetController` (`self.MyEmemy`))))
  (bind _blackboardcomponent (`AIController.UseBlackboard` _asbp_ai_enemy_controller "/Game/Blueprint/enemy_AI_BP/BB_ENEMY_BEHAVIOR.BB_ENEMY_BEHAVIOR"))
  (`KismetSystemLibrary.PrintString` (`KismetStringLibrary.Conv_VectorToString` _returnvalue) true true (struct :`G` 0.66 :`B` 1.0 :`A` 1.0) 10.0)
  (`BlackboardComponent.SetValueAsVector` _blackboardcomponent "PlayerLocation" _returnvalue))

(fn `UserConstructionScript`)