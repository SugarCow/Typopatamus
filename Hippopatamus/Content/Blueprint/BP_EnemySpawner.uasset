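; Enemy spawner actor that places a BP_ENEMY1 at its own location when play begins.
; BeginPlay casts the first player controller to BP_PlayerController and stores itself there as MyEnemySpawner, then calls SpawnEnemy.
; If the cast fails, nothing spawns.
; SpawnEnemy is a separate function that performs a single spawn, with an unconnected debug print left in its graph.
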(event `self.ReceiveBeginPlay`
  (bind _asbp_player_controller (cast `/Game/Blueprint/BP_PlayerController` (`GameplayStatics.GetPlayerController` 0)))
  (set `/Game/Blueprint/BP_PlayerController.MyEnemySpawner` self _asbp_player_controller)
  (`self.SpawnEnemy`))

(fn `SpawnEnemy`
  (`|SpawnActorFromClass` "/Game/Blueprint/BP_ENEMY1.BP_ENEMY1_C" (`KismetMathLibrary.MakeTransform` (`self.K2_GetActorLocation`)) "Undefined" "OverrideRootScale" null null))

(fn `UserConstructionScript`)