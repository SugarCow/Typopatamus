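; Behavior Tree task that sends the enemy AI's pawn to the player location stored in the Blackboard.
; It skips the move if the pawn is already within a small tolerance of that point, otherwise it calls AIMoveTo.
; Both paths finish successfully after a fixed Delay, which starts when the move is issued and ignores its result.
; Debug prints show both locations and when movement starts.
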(event `self.ReceiveExecute`
  (params (OwnerActor :type "Actor Object Reference"))
  (bind _returnvalue (`BTFunctionLibrary.GetBlackboardValueAsVector` (`self.myPlayerLocation`)))
  (bind _asbp_ai_enemy_controller (cast `/Game/Blueprint/enemy_AI_BP/BP_AI_ENEMY_CONTROLLER` OwnerActor))
  (`KismetSystemLibrary.PrintString` (`KismetStringLibrary.Concat_StrStr` "Player Location: " (`KismetStringLibrary.Conv_VectorToString` _returnvalue)) true true (struct :`G` 0.66 :`B` 1.0 :`A` 1.0) 15.0)
  (bind _returnvalue_2 (`Controller.K2_GetPawn` _asbp_ai_enemy_controller))
  (bind _returnvalue_3 (`Actor.K2_GetActorLocation` _returnvalue_2))
  (`KismetSystemLibrary.PrintString` (`KismetStringLibrary.Concat_StrStr` "Enemy Location" (`KismetStringLibrary.Conv_VectorToString` _returnvalue_3)) true true (struct :`G` 0.66 :`B` 1.0 :`A` 1.0) 15.0)
  (if (not (== _returnvalue _returnvalue_3 :`ErrorTolerance` 10.0))
    (`KismetSystemLibrary.PrintString` "moving")
    (`|AIMoveTo` _returnvalue_2 _returnvalue null 1.0
      (:`then`
        _)))
  (`KismetSystemLibrary.Delay` 10.0)
  (`self.FinishExecute` true))