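; BP_Enemy is an enemy Blueprint that moves itself along world +X by MovementSpeed every Tick unless StopMoving is set.
; Movement is a per-frame SetActorLocation without sweep or delta-time scaling, printing each new position as debug output.
; The SwitchDriectionCollisionBox overlap checks for BP_Tile1 but takes no action, so direction switching is unfinished.
; SpawnEnemy is empty, and unconnected AI move and stop nodes never run.
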(event `self.ReceiveTick`
  (params (DeltaSeconds :type "Float (single-precision)"))
  (bind _returnvalue (+ (`KismetMathLibrary.MakeVector` (`self.MovementSpeed`)) (`self.K2_GetActorLocation`)))
  (if (not (`self.stopMoving`))
    (`KismetSystemLibrary.PrintString` (`KismetStringLibrary.Conv_VectorToString` _returnvalue))
    (`self.K2_SetActorLocation` _returnvalue)))

(event `self.switchDriectionCollisionBox.OnComponentBeginOverlap`
  (params (OverlappedComponent :type "PrimitiveComponent Object Reference") (OtherActor :type "Actor Object Reference") (OtherComp :type "PrimitiveComponent Object Reference") (OtherBodyIndex :type Integer) (bFromSweep :type Boolean) (SweepResult :type "HitResult Structure (by ref)"))
  (cast `/Game/Blueprint/BP_Tile1` OtherActor)
  (if true
    _))

(fn `SpawnEnemy`)

(fn `UserConstructionScript`)