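; BP_ENEMY1 is an enemy actor that pairs itself with the player and takes on an AI controller when play begins.
; On BeginPlay it casts the player pawn to BP_Player, stores it, then spawns BP_AI_ENEMY_CONTROLLER at its own location to possess it.
; It then registers itself in the player's MyEmemy variable, with debug prints along the way.
; The closing Delay leads nowhere, and Tick and overlap events are empty.
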(event `self.ReceiveBeginPlay`
  (bind _returnvalue (`GameplayStatics.GetPlayerPawn` 0))
  (bind _myplayer (`self.MyPlayer`))
  (`KismetSystemLibrary.PrintString` (`KismetSystemLibrary.GetDisplayName` _returnvalue))
  (bind _asbp_player (cast `/Game/Blueprint/BP_Player` _returnvalue))
  (set `self.MyPlayer` _asbp_player)
  (bind _returnvalue_2 (`|SpawnActorFromClass` "/Game/Blueprint/enemy_AI_BP/BP_AI_ENEMY_CONTROLLER.BP_AI_ENEMY_CONTROLLER_C" (`KismetMathLibrary.MakeTransform` (`self.K2_GetActorLocation`)) "Undefined" "OverrideRootScale" null null))
  (`Controller.Possess` _returnvalue_2 self)
  (set `/Game/Blueprint/BP_Player.MyEmemy` self _myplayer)
  (`KismetSystemLibrary.PrintString` (`KismetSystemLibrary.GetDisplayName` (`/Game/Blueprint/BP_Player.MyEmemy` _myplayer)))
  (`KismetSystemLibrary.Delay` 10.0))

(event `self.ReceiveTick`
  (params (DeltaSeconds :type "Float (single-precision)")))

(fn `UserConstructionScript`)